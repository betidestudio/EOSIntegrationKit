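; Player controller for an Epic Online Services (EIK) multiplayer game that handles lobby presentation and moves lobby players into a matchmaking session.
; On BeginPlay it sets a cine camera and fade on the lobby map, or game-only input on the session map.
; A session code goes through a server event to every player in the GameMode's list.
; Each client finds that session by key, destroys its current one and joins, only printing the result.
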(event Custom|AddPlayerWidget
  (Utilities|FlowControl|DoOnce false
    (:Completed
      (bind _returnvalue (UserInterface|CreateWidget "/EOSIntegrationKit/EIK_ExampleContent/Widgets/Lobby/WBP_Lobby.WBP_Lobby_C"))
      (UserInterface|Viewport|AddtoViewport _returnvalue 1))))

(event Custom|DistributeSessionCode
  (params (Session%20Code :type String))
  (CallFunction|ServerDistributeSessionCode Session%20Code))

(event Custom|Server_DistributeSessionCode
  (params (Session%20Code :type String))
  (bind _asbp_third_person_game_mode (Utilities|Casting|CastToBP_ThirdPersonGameMode (Game|GetGameMode)))
  (for _array_element (Variables|/EOSIntegrationKit/EIK_ExampleContent/EpicContent/ThirdPerson/Blueprints/BP_ThirdPersonGameMode.BP_ThirdPersonGameMode_C|GetPlayerList _asbp_third_person_game_mode)
    (CallFunction|OwningClientGetSessionCode _array_element Session%20Code)))

(event Custom|OwningClient_GetSessionCode
  (params (Session%20Code :type String))
  (bind _sessionresults (|FindEIKSessions (Utilities|Map|MakeMap "SessionKey" (Utilities|Struct|MakeEIKAttribute "String" Session%20Code false)) "MT_MatchMakingSession" 15 "RE_NoSelection" false)
    (:OnSuccess
      (if (Utilities|Array|IsValidIndex _sessionresults)
        (|DestroySession (Game|GetPlayerController 0)
          (:OnSuccess
            _)
          (:OnFailure
            _))
        (bind _sessionjoinaddress (|JoinEIKSessions (Utilities|Array|Get(acopy) _sessionresults))
          (:OnSuccess
            (Development|PrintString _sessionjoinaddress))
          (:OnFail
            (Development|PrintString "Join EIK Failed")))))))

(event EventBeginPlay
  (bind _returnvalue (Game|GetCurrentLevelName true))
  (switch string _returnvalue
    (:LobbyMap
      ;[1 1 1] Just for test
      (Utilities|FlowControl|Delay 4.0)
      (bind _outactors (Actor|GetAllActorsOfClass "/Script/CinematicCamera.CineCameraActor"))
      (Game|Player|SetViewTargetwithBlend (Utilities|Array|Get(acopy) _outactors) 0.0 "VTBlend_Linear" 0.0 false)
      (CameraFades|StartCameraFade :self (Variables|Default|GetPlayerCameraManager) :FromAlpha 1.0 :Duration 4.0 :bHoldWhenFinished true))
    (:SessionMap
      (if (Pawn|IsLocalController)
        (Input|SetInputModeGameOnly self false)
        (Variables|Default|SetbShowMouseCursor false)))))

(fn ConstructionScript)